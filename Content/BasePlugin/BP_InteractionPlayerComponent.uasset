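; Player interaction component that finds interactable components in front of its owner and drives hold interactions on them.
; Outside a hold, Tick line-traces from a base component and caches hits implementing DMK_InteractionTargetInterface; during one, it accumulates hold time.
; Hold events forward start, stop and orientation-corrected axis input to the target, which can also be set directly.
; Targets can request an interaction input mapping context and movement lock, and supply description and icon.
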(event Custom|SetComponentToHold
  (params (CachedComponent :type Primitive%20Component%20Object%20Reference) (Issuer :type Actor%20Object%20Reference))
  (Utilities|IsValid (Variables|Default|GetCachedComponent)
    (:Is%20Valid
      (CallFunction|HoldInteractionStop Issuer (Variables|Default|GetTimeElapsed)))
    (:Is%20Not%20Valid
      _))
  (Variables|Default|SetCachedComponent CachedComponent)
  (CallFunction|HoldInteraction Issuer))

(event EventBeginPlay)

(event EventTick
  (params (DeltaSeconds :type Float%20%28single-precision%29))
  (if (not (Variables|Default|GetDuringHoldingInteraction))
    (CallFunction|UpdateInteractionTarget)
    (else
      (Variables|Default|SetTimeElapsed (+ DeltaSeconds (Variables|Default|GetTimeElapsed))))))

(event EventHoldInteractionStop
  (params (Issuer :type Actor%20Object%20Reference) (TimeElapsed :type Float%20%28single-precision%29))
  (Variables|Default|SetDuringHoldingInteraction false)
  (Utilities|IsValid (Variables|Default|GetCachedComponent)
    (:Is%20Valid
      (bind _returnvalue (Class|DMKInteractionTargetInterface|GetInputMapping(Message) (Variables|Default|GetCachedComponent)))
      (if (Utilities|IsValidSoftObjectReference _returnvalue)
        (Input|RemoveMappingContext (PlayerController|LocalPlayerSubsystems|GetEnhancedInputLocalPlayerSubsystem (Game|GetPlayerController 0)) "/DMK_MouseAxisInteraction/Inputs/Interactions/IMC_DMK_Interaction.IMC_DMK_Interaction" "(bIgnoreAllPressedKeysUntilRelease=True,bForceImmediately=False,bNotifyUserSettings=False)")
        (Variables|Default|SetMappingAdded false)
        (Class|DMKInteractionTargetInterface|HoldInteractionStop(Message) (Variables|Default|GetCachedComponent) (Components|GetOwner) TimeElapsed)
        (bind _returnvalue_2 (Class|DMKInteractionTargetInterface|ShouldBlockMovement(Message) (Variables|Default|GetCachedComponent)))
        (if _returnvalue_2
          (CallFunction|SetMovementState))
        (else
          (Class|DMKInteractionTargetInterface|HoldInteractionStop(Message) (Variables|Default|GetCachedComponent) (Components|GetOwner) TimeElapsed))))))

(event EventHoldInteraction
  (params (Issuer :type Actor%20Object%20Reference))
  (bind _cachedcomponent (Variables|Default|GetCachedComponent))
  (Utilities|IsValid (Variables|Default|GetCachedComponent)
    (:Is%20Valid
      (Variables|Default|SetDuringHoldingInteraction true)
      (Variables|Default|SetTimeElapsed 0.0)
      (bind _returnvalue (Class|DMKInteractionTargetInterface|GetInputMapping(Message) (Variables|Default|GetCachedComponent)))
      (if (Utilities|IsValidSoftObjectReference _returnvalue)
        (if (not (Variables|Default|GetMappingAdded))
          (Input|AddMappingContext (PlayerController|LocalPlayerSubsystems|GetEnhancedInputLocalPlayerSubsystem (Game|GetPlayerController 0)) "/DMK_MouseAxisInteraction/Inputs/Interactions/IMC_DMK_Interaction.IMC_DMK_Interaction" 1 "(bIgnoreAllPressedKeysUntilRelease=True,bForceImmediately=False,bNotifyUserSettings=False)")
          (Variables|Default|SetMappingAdded true)
          (Class|DMKInteractionTargetInterface|HoldInteraction(Message) _cachedcomponent (Components|GetOwner))
          (bind _returnvalue_2 (Class|DMKInteractionTargetInterface|ShouldBlockMovement(Message) _cachedcomponent))
          (if _returnvalue_2
            (CallFunction|SetMovementState)))
        (else
          (Class|DMKInteractionTargetInterface|HoldInteraction(Message) (Variables|Default|GetCachedComponent) (Components|GetOwner)))))))

(event EventHoldInteractionAxis
  (params (Issuer :type Actor%20Object%20Reference) (Axis :type Vector%202D%20Structure%20%28by%20ref%29))
  (Utilities|IsValid (Variables|Default|GetCachedComponent)
    (:Is%20Valid
      (Class|DMKInteractionTargetInterface|HoldInteractionAxis(Message) (Variables|Default|GetCachedComponent) (Components|GetOwner) (* Axis (* (Math|Float|Sign(Float) (Math|Vector|DotProduct (Transformation|GetActorRightVector (Components|GetOwner)) (Transformation|GetActorForwardVector (Components|GetOwner (Variables|Default|GetCachedComponent))))) -1.0))))))

(fn UpdateInteractionTarget
  (bind _interactionbasecomponent (Variables|Default|GetInteractionBaseComponent))
  (bind _returnvalue (Transformation|GetWorldLocation _interactionbasecomponent))
  (Utilities|IsValid (Variables|Default|GetInteractionBaseComponent)
    (:Is%20Valid
      (bind (_outhit _returnvalue_2) (Collision|LineTraceByChannel _returnvalue (+ (* (Math|Vector|GetForwardVector (Variables|Default|GetInteractionBaseComponent)) 3e+02) _returnvalue) "TraceTypeQuery1" false 0 (select (Variables|Default|GetShowTrace) "ForOneFrame" "None") (Variables|Default|GetShouldIgnoreOwner)))
      (if _returnvalue_2
        (if (Utilities|DoesObjectImplementInterface (.HitComponent (Collision|BreakHitResult _outhit)) "/Script/DMK_MouseAxisInteraction.DMK_InteractionTargetInterface")
          (Variables|Default|SetCachedComponent (.HitComponent (Collision|BreakHitResult _outhit)))
          (Variables|Default|SetHitLocation (.Location (Collision|BreakHitResult _outhit)))
          (else
            (Variables|Default|SetCachedComponent 0 :!label _label)
            (if (Variables|Default|GetMappingAdded)
              (Input|RemoveMappingContext (PlayerController|LocalPlayerSubsystems|GetEnhancedInputLocalPlayerSubsystem (Game|GetPlayerController 0)) "/DMK_MouseAxisInteraction/Inputs/Interactions/IMC_DMK_Interaction.IMC_DMK_Interaction" "(bIgnoreAllPressedKeysUntilRelease=True,bForceImmediately=False,bNotifyUserSettings=False)")
              (Variables|Default|SetMappingAdded false))))
        (else
          (goto _label))))))

(fn SetMovementState
  (bind _returnvalue (Components|GetOwner))
  (bind _returnvalue_2 (Actor|GetComponentbyClass _returnvalue "/Script/Engine.CharacterMovementComponent"))
  (if (Variables|Default|GetMappingAdded)
    (Pawn|Components|CharacterMovement|SetMovementMode _returnvalue_2 "MOVE_None" 0)
    (else
      (Pawn|Components|CharacterMovement|SetMovementMode _returnvalue_2 "MOVE_Walking" 0))))

(fn GetInputMapping
  (return 0))

(fn GetInteractionDescription
  (bind _cachedcomponent (Variables|Default|GetCachedComponent))
  (Utilities|IsValid _cachedcomponent
    (:Is%20Valid
      (bind _returnvalue (Class|DMKInteractionTargetInterface|GetInteractionDescription(Message) _cachedcomponent))
      (return _returnvalue))))

(fn GetInteractionIcon
  (bind _cachedcomponent (Variables|Default|GetCachedComponent))
  (Utilities|IsValid _cachedcomponent
    (:Is%20Valid
      (bind _returnvalue (Class|DMKInteractionTargetInterface|GetInteractionIcon(Message) _cachedcomponent))
      (return _returnvalue))))

(fn HasInputMapping
  (return false))

(fn ShouldBlockMovement
  (return false))