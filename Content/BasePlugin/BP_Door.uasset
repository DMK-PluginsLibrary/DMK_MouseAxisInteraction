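; Physics-driven door that is pushed or dragged through DMK interaction components on the door and its front knob.
; A press applies an impulse signed by the issuer's orientation, while held axis input applies force along the door's right vector.
; Horizontal-dominant knob input turns the handle within clamped limits, and vertical input moves the door.
; Knob and door angles together toggle Closed, which switches physics simulation off to latch the door.
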(event PressInteraction(DMK_DoorInteraction)
  (params (Issuer :type Actor%20Object%20Reference))
  (if (Physics|IsSimulatingPhysics (Variables|Default|GetDoor) "None")
    (Physics|AddImpulse (Variables|Default|GetDoor) (* (Math|Vector|GetRightVector (Variables|Default|GetDoor)) (Variables|Default|GetSinglePushForce) (* (Math|Float|Sign(Float) (Math|Vector|DotProduct (Transformation|GetActorForwardVector) (Transformation|GetActorRightVector Issuer))) -1.0)) "None" false)
    (Development|PrintString "Interaction")))

(event HoldInteractionStopEvent(DMK_KnobInteractionFront)
  (params (Issuer :type Actor%20Object%20Reference) (TimeElapsed :type Float%20%28single-precision%29))
  (Variables|Default|SetbHoldingKnob false)
  (Variables|Default|SetbKnobClosed false))

(event HoldInteractionEvent(DMK_KnobInteractionFront)
  (params (Issuer :type Actor%20Object%20Reference))
  (Variables|Default|SetbHoldingKnob true))

(event HoldAxisInteractionEvent(DMK_DoorInteraction)
  (params (Issuer :type Actor%20Object%20Reference) (Axis :type Vector%202D%20Structure%20%28by%20ref%29))
  (CallFunction|DoorAxisPhysicalMovement Axis))

(event HoldInteractionEvent(DMK_DoorInteraction)
  (params (Issuer :type Actor%20Object%20Reference)))

(event HoldAxisInteractionEvent(DMK_KnobInteractionFront)
  (params (Issuer :type Actor%20Object%20Reference) (Axis :type Vector%202D%20Structure%20%28by%20ref%29))
  (bind (_x _y) (Math|Vector2D|BreakVector2D Axis))
  (bind _scene (Variables|Default|GetScene))
  (bind _relativerotation (Variables|/Script/Engine.SceneComponent|GetRelativeRotation _scene))
  (bind (_roll _pitch _yaw) (Math|Rotator|BreakRotator _relativerotation))
  (Utilities|FlowControl|Sequence
    (:then_0
      (if (> (Math|Float|Absolute(Float) _x) (Math|Float|Absolute(Float) _y))
        (Transformation|SetRelativeRotation (Variables|Default|GetScene) (Math|Rotator|MakeRotator _roll (Math|Float|ClampAngle (+ (* _x (Math|Float|Sign(Float) (Math|Vector|DotProduct (Transformation|GetActorForwardVector Issuer) (Math|Vector|GetRightVector (Variables|Default|GetDoor))))) _pitch) 0.0 9e+01) _yaw) false false)
        (Utilities|FlowControl|Sequence
          (:then_0
            (Variables|Default|SetbKnobClosed (Math|Float|NearlyEqual(Float) (.Pitch (Math|Rotator|BreakRotator (Variables|/Script/Engine.SceneComponent|GetRelativeRotation (Variables|Default|GetScene)))) 0.0 0.1)))
          (:then_1
            (if (and (Variables|Default|GetbKnobClosed) (Math|Float|NearlyEqual(Float) (.Yaw (Math|Rotator|BreakRotator (Variables|/Script/Engine.SceneComponent|GetRelativeRotation (Variables|Default|GetDoor)))) -9e+01 0.1))
              (if (not (Variables|Default|GetClosed))
                (Variables|Default|SetClosed true)
                (Physics|SetSimulatePhysics (Variables|Default|GetDoor) false))
              (elif (Variables|Default|GetClosed)
                (Variables|Default|SetClosed false)
                (Physics|SetSimulatePhysics (Variables|Default|GetDoor) true)))))
        (else
          (Utilities|FlowControl|DelayUntilNextTick)
          (CallFunction|DoorAxisPhysicalMovement (Math|Vector2D|MakeVector2D 0.0 _y)))))))

(event EventBeginPlay
  (Physics|SetSimulatePhysics (Variables|Default|GetDoor) (not (Variables|Default|GetClosed))))

(event Collision|EventActorBeginOverlap
  (params (OtherActor :type Actor%20Object%20Reference)))

(event EventTick
  (params (DeltaSeconds :type Float%20%28single-precision%29)))

(fn ConstructionScript)

(fn DoorAxisPhysicalMovement
  (params (InVec :type Vector%202D%20Structure))
  (bind (_x _y) (Math|Vector2D|BreakVector2D InVec))
  (if (Physics|IsSimulatingPhysics (Variables|Default|GetDoor) "None")
    (Physics|AddForce (Variables|Default|GetDoor) (* (Variables|Default|GetFinalForceMultiplier) (* (+ _x _y) (Variables|Default|GetAxisMultiplier)) (Math|Vector|GetRightVector (Variables|Default|GetDoor))) "None" false)))